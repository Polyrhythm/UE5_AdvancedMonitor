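; BP_Monitor is an actor that applies image-monitoring overlays, either a waveform or false color, through its MonitorPP post process settings.
; The construction script branches on the Monitor enum and creates a dynamic material instance, configured from WaveformParams (RGB parade, tint, box position, opacity) or FalseColorParams (visualization map).
; That instance becomes the post process blendable, while the default mode assigns no material.
; The event graph holds no active logic.
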(fn `UserConstructionScript`
  (bind _waveform_params_isrgbparade (break `/AdvancedMonitor/Monitors/ST_WaveformParams` (`self.Waveform Params`)))
  (bind (_waveform_params_isrgbparade_2 _waveform_params_waveformtint _waveform_params_boxposition _waveform_params_opacity) (break `/AdvancedMonitor/Monitors/ST_WaveformParams` (`self.Waveform Params`)))
  (bind (_waveform_params_isrgbparade_3 _waveform_params_waveformtint_2) (break `/AdvancedMonitor/Monitors/ST_WaveformParams` (`self.Waveform Params`)))
  (bind _falsecolorparams_falsecolormap (break `/AdvancedMonitor/Monitors/ST_FalseColorParams` (`self.FalseColorParams`)))
  (bind _settings (`PostProcessComponent.Settings` (`self.Monitor_PP`)))
  (if (`|EnumEquality` (`self.Monitor`) "NewEnumerator0")
    ;[1 1 1] Waveform
    (bind _returnvalue (`KismetMaterialLibrary.CreateDynamicMaterialInstance` (`self.M_Waveform`)))
    (`MaterialInstanceDynamic.SetScalarParameterValue` _returnvalue "IsRGBParade" (`KismetMathLibrary.Conv_BoolToDouble` _waveform_params_isrgbparade))
    (`MaterialInstanceDynamic.SetVectorParameterValue` _returnvalue "Waveform Tint" (`KismetMathLibrary.Conv_ColorToLinearColor` _waveform_params_waveformtint_2))
    (`MaterialInstanceDynamic.SetVectorParameterValue` _returnvalue "Position (XY MAX, ZW MIN)" (`KismetMathLibrary.Conv_ColorToLinearColor` _waveform_params_boxposition))
    (`MaterialInstanceDynamic.SetScalarParameterValue` _returnvalue "Opacity" _waveform_params_opacity)
    (setmembers `PostProcessSettings` :`StructRef` _settings :`WeightedBlendables` (make `WeightedBlendables` (`|MakeArray` (make `WeightedBlendable` 1.0 _returnvalue))))
    (elif (`|EnumEquality` (`self.Monitor`) "NewEnumerator1")
      ;[1 1 1] False Color
      (bind _returnvalue_2 (`KismetMaterialLibrary.CreateDynamicMaterialInstance` (`self.M_FalseColor`)))
      (`MaterialInstanceDynamic.SetScalarParameterValue` _returnvalue_2 "Visualization Map" (`KismetMathLibrary.Conv_IntToDouble` (`KismetMathLibrary.Conv_ByteToInt` _falsecolorparams_falsecolormap)))
      (setmembers `PostProcessSettings` :`StructRef` (`PostProcessComponent.Settings` (`self.Monitor_PP`)) :`WeightedBlendables` (make `WeightedBlendables` (`|MakeArray` (make `WeightedBlendable` 1.0 _returnvalue_2))))
      (elif (`|EnumEquality` (`self.Monitor`) "NewEnumerator2")
        ;[1 1 1] Default (no materials)
        (setmembers `PostProcessSettings` :`StructRef` _settings :`WeightedBlendables` (make `WeightedBlendables` (`|MakeArray` (struct) :!type "WeightedBlendable Structure")))))))